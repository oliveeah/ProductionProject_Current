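; BP_TestCharacter is a test player character for trying out delegates, interfaces, montages and widget calls.
; On BeginPlay it binds a custom event to every BP_DelegateSender's AddCard delegate, forwarding it to the player widget's WidgetAddCardNew.
; Construction applies MovementSpeed to max walk speed.
; A self-restarting hold-montage event exists, but its toggle, axe attack and widget creation are disconnected, and the overlap interface check does nothing.
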(event `CustomEvent`
  (`|PlayMontage` (`self.Mesh`) "/Game/Characters/Mannequins/Anims/hold_montage.hold_montage"
    (:`OnBlendOut`
      (`self.CustomEvent`))))

(event `Key|LeftMouseButton`
  (params (Key :type "Key Structure")))

(event `self.ReceiveActorBeginOverlap`
  (params (OtherActor :type "Actor Object Reference"))
  (if (`KismetSystemLibrary.DoesImplementInterface` OtherActor "/Script/ProductionProjCurr.testInterface")
    _))

(event `self.ReceiveBeginPlay`
  (bind _outactors (`GameplayStatics.GetAllActorsOfClass` "/Game/RefactoredStuff/Blueprints/delegateSender_PROTOTYPE/BP_DelegateSender.BP_DelegateSender_C"))
  (for _array_element _outactors
    (add `/Game/RefactoredStuff/Blueprints/delegateSender_PROTOTYPE/BP_DelegateSender.addCardDelegate` _array_element (delegate `playerTestCustomEvent`)))
  (`KismetSystemLibrary.PrintString` "player listening to delegate(s)" true true (struct :`R` 0.038162 :`G` 0.319792 :`A` 1.0)))

(event `playerTestCustomEvent`
  (`/Game/MyStuff/Blueprints/UI/Player_Widget.widgetAddCardNew` (`self.PlayerWidgetRef`)))

(fn `UserConstructionScript`
  (set `CharacterMovementComponent.MaxWalkSpeed` (`self.movementSpeed`) (`self.CharacterMovement`)))